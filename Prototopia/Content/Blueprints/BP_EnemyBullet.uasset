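; Enemy projectile Blueprint that damages the first-person player character when its Bullet component begins overlapping them.
; A raised shield absorbs the hit, losing one ShieldHP; once depleted, it is removed, hidden and moved to its lowered point.
; Otherwise the player loses one HP, and dropping below one opens FirstPersonMap.
; The graph writes character state directly and contains no movement or self-destroy logic.
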(event `self.Bullet.OnComponentBeginOverlap`
  (params (OverlappedComponent :type "PrimitiveComponent Object Reference") (OtherActor :type "Actor Object Reference") (OtherComp :type "PrimitiveComponent Object Reference") (OtherBodyIndex :type Integer) (bFromSweep :type Boolean) (SweepResult :type "HitResult Structure (by ref)"))
  (bind _asbp_first_person_character (cast `/Game/Blueprints/BP_FirstPersonCharacter` OtherActor))
  (if (`/Game/Blueprints/BP_FirstPersonCharacter.ShieldRaised` _asbp_first_person_character)
    (bind _output_get (set `/Game/Blueprints/BP_FirstPersonCharacter.ShieldHP` (- (`/Game/Blueprints/BP_FirstPersonCharacter.ShieldHP` _asbp_first_person_character) 1.0) _asbp_first_person_character))
    (if (< _output_get 1.0)
      (set `/Game/Blueprints/BP_FirstPersonCharacter.HasShield` false _asbp_first_person_character)
      (`SceneComponent.SetVisibility` (`/Game/Blueprints/BP_FirstPersonCharacter.SM_Shield` _asbp_first_person_character) false false)
      (bind _shieldloweredpoint (`/Game/Blueprints/BP_FirstPersonCharacter.ShieldLoweredPoint` _asbp_first_person_character))
      (`KismetSystemLibrary.MoveComponentTo` (`/Game/Blueprints/BP_FirstPersonCharacter.SM_Shield` _asbp_first_person_character) (`SceneComponent.RelativeLocation` _shieldloweredpoint) (`SceneComponent.RelativeRotation` _shieldloweredpoint) false false 0.1)
      (set `/Game/Blueprints/BP_FirstPersonCharacter.ShieldRaised` false _asbp_first_person_character))
    (else
      (bind _output_get_2 (set `/Game/Blueprints/BP_FirstPersonCharacter.HP` (- (`/Game/Blueprints/BP_FirstPersonCharacter.HP` _asbp_first_person_character) 1.0) _asbp_first_person_character))
      (if (< _output_get_2 1.0)
        (`GameplayStatics.OpenLevel` "FirstPersonMap")))))

(fn `UserConstructionScript`)