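; Enemy gun turret that turns toward pawns it sees and fires bullets from two barrels.
; Each PawnSensing sighting snaps the turret top's yaw using a look-at rotation from pawn to turret with an offset, applied as relative rotation.
; Chained Delays then stagger BP_EnemyBullet spawns at each barrel's transform, pacing fire because repeat sightings do not restart a pending Delay.
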(event `self.PawnSensing.OnSeePawn`
  (params (Pawn :type "Pawn Object Reference"))
  (bind (_returnvalue_roll _returnvalue_pitch _returnvalue_yaw) (`KismetMathLibrary.BreakRotator` (`KismetMathLibrary.FindLookAtRotation` (`self.K2_GetActorLocation` Pawn) (`SceneComponent.K2_GetComponentLocation` (`self.GunTurretTop`)))))
  (`SceneComponent.K2_SetRelativeRotation` (`self.GunTurretTop`) (`KismetMathLibrary.MakeRotator` 0.0 0.0 (- _returnvalue_yaw 90.0)) false false)
  (`KismetSystemLibrary.Delay` 1.2)
  (`|SpawnActorFromClass` "/Game/Blueprints/BP_EnemyBullet.BP_EnemyBullet_C" (`SceneComponent.K2_GetComponentToWorld` (`self.Barrel`)) "AlwaysSpawn" "MultiplyWithRoot" null null)
  (`KismetSystemLibrary.Delay` 0.8)
  (`|SpawnActorFromClass` "/Game/Blueprints/BP_EnemyBullet.BP_EnemyBullet_C" (`SceneComponent.K2_GetComponentToWorld` (`self.Barrel1`)) "AlwaysSpawn" "MultiplyWithRoot" null null))

(fn `UserConstructionScript`)